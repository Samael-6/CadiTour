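; GM_Voiture, apparently a game mode, gives each shelf actor (BP_Etageres) in the level a random product.
; On BeginPlay it caches every shelf in ListeEtagere.
; The AssignationAlimentaire event rerolls a random index into Produits until it is absent from ProductTaken, then sets the shelf's Produit and records the index.
; The reroll has no exit if shelves outnumber available products.
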(event Custom|AssignationAlimentaire
  (for _array_element (Variables|Default|GetListeEtagere)
    (Variables|Default|SetIndexProduct (Math|Random|RandomIntegerinRange 0 (Utilities|Array|LastIndex (Variables|Default|GetProduits))) :!label _label)
    (for _array_element_2 (Variables|Default|GetProductTaken)
      (if (== _array_element_2 (Variables|Default|GetIndexProduct))
        (goto _label)))
    (Variables|/Game/Game/BP_Etageres.BP_Etageres_C|SetProduit _array_element (Utilities|Array|Get(acopy) (Variables|Default|GetProduits) (Variables|Default|GetIndexProduct)))
    (Utilities|Array|Add (Variables|Default|GetProductTaken) (Variables|Default|GetIndexProduct))))

(event EventBeginPlay
  (bind _outactors (Actor|GetAllActorsOfClass "/Game/Game/BP_Etageres.BP_Etageres_C"))
  (Variables|Default|SetListeEtagere _outactors))

(fn ConstructionScript)